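; Enemy pickup-style actor that changes the player's health on contact.
; When its Box overlaps a BP_ThirdPersonCharacter, the givePoints event passes PointsToGive to the character's AffectHealth and destroys the actor.
; The construction script gives the Cube a dynamic BasicShapeMaterial instance tinted by the Color variable.
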(event OnComponentBeginOverlap(Box)
  (params (OverlappedComponent :type Primitive%20Component%20Object%20Reference) (OtherActor :type Actor%20Object%20Reference) (OtherComp :type Primitive%20Component%20Object%20Reference) (OtherBodyIndex :type Integer) (bFromSweep :type Boolean) (SweepResult :type Hit%20Result%20Structure%20%28by%20ref%29))
  (bind _asbp_third_person_character (Utilities|Casting|CastToBP_ThirdPersonCharacter OtherActor))
  (CallFunction|Givepoints _asbp_third_person_character))

(event Custom|givePoints
  (params (personaje :type BP%20Third%20Person%20Character%20Object%20Reference))
  ;[1 1 1] dar 1 punto al jugador
  (Default|AffectHealth personaje (Variables|Default|GetpointsToGive))
  (Actor|DestroyActor))

(fn ConstructionScript
  (bind _returnvalue (Rendering|Material|CreateDynamicMaterialInstance (Variables|Default|GetCube) 0 "/Engine/BasicShapes/BasicShapeMaterial.BasicShapeMaterial" "None" :!class /Script/Engine.PrimitiveComponent))
  (Rendering|Material|SetVectorParameterValue _returnvalue "Color" (Variables|Default|Getcolor) :!class /Script/Engine.MaterialInstanceDynamic))